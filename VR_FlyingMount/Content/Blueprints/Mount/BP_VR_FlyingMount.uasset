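; VR flying mount that a player grabs to ride, with flight movement not defined in this graph.
; Grabbing stores the hand, makes its owner the mount's Owner and attaches that actor to the mount; release only clears the hand.
; Throttle is polled from the holding hand's owner via GetThrottleMessage, while GetThrottle is a stub returning zero.
; The trigger value is inverted into CanRoll, so pressing it disables roll.
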(event EventBeginPlay)

(event Collision|EventActorBeginOverlap
  (params (OtherActor :type Actor%20Object%20Reference)))

(event Event_Trigger
  (params (Trigger_Pressed :type Integer))
  ;[1 1 1] Invert the trigger pressed value and set Can Roll to that value.
  (Class|FlyingMountBase|SetCanRoll (Math|Conversions|ToBoolean(Integer) (- 1 Trigger_Pressed))))

(fn ConstructionScript)

(fn GetThrottleValue
  (bind _holdinghand (Variables|Default|GetHoldingHand))
  (Utilities|IsValid _holdinghand
    (:Is%20Valid
      (bind _throttle_value (Class|BPIVRInteraction|GetThrottle(Message) (Components|GetOwner _holdinghand)))
      (return _throttle_value))
    (:Is%20Not%20Valid
      (return 0.0))))

(fn GetThrottle
  (return 0.0))

(fn Grab
  (params (Grabbing_Hand :type Scene%20Component%20Object%20Reference) (Grabbed :type Boolean))
  ;[1 1 1] If we get a Grab message that is true, set the Holding Hand to the object that is grabbing us, set our Owner to the owner of the Holding Hand, and attach the Owner of the holding hand to us.
  ; If we are not Grabbed, clear the Holding Hand and Owner.
  (if Grabbed
    (bind _output_get (Variables|Default|SetHoldingHand Grabbing_Hand))
    (Actor|SetOwner (Components|GetOwner _output_get))
    (Transformation|AttachActorToActor (Components|GetOwner _output_get) self "None" "KeepWorld" "KeepWorld" "KeepWorld" true)
    (return true)
    (else
      (Variables|Default|SetHoldingHand 0)
      (return false))))